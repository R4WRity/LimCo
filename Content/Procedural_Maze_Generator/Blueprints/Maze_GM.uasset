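; Game mode for the procedural maze generator that handles in-game editing of walls and the exit.
; While Edit is on, Tick sphere-traces along the edit controller camera, caches the targeted cell and wall, and draws a color-coded debug sphere.
; Remove, create and place-exit events apply changes to that cell and write them back to the Maze's wall parameters or exit index.
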(event `self.ReceiveTick`
  (params (DeltaSeconds :type "Float (single-precision)"))
  (if (`self.Edit`)
    (bind _outactors (`GameplayStatics.GetAllActorsOfClass` (`self.DefaultPawnClass`)))
    (bind _returnvalue (`self.K2_GetActorLocation` (`|GetArrayItem` _outactors)))
    (bind (_outhit _returnvalue_2) (`KismetSystemLibrary.SphereTraceSingle` _returnvalue (+ _returnvalue (* (`SceneComponent.GetForwardVector` (`/Game/Procedural_Maze_Generator/Blueprints/MazeEditController.Camera` (cast `/Game/Procedural_Maze_Generator/Blueprints/MazeEditController` (`GameplayStatics.GetPlayerController` 0) :!pure true))) 2000.0)) 24.0 "TraceTypeQuery1"))
    (if _returnvalue_2
      (bind (_bblockinghit _binitialoverlap _time _distance _location _impactpoint _normal _impactnormal _physmat _hitactor _hitcomponent) (`GameplayStatics.BreakHitResult` _outhit))
      (bind _ascell_bp (cast `/Game/Procedural_Maze_Generator/Blueprints/Cell_BP` _hitactor))
      (set `self.Cell` _ascell_bp)
      (bind _returnvalue_3 (!= _hitcomponent (`/Game/Procedural_Maze_Generator/Blueprints/Cell_BP.Floor` _ascell_bp)))
      (if _returnvalue_3
        (set `self.Component` _hitcomponent))
      (`KismetSystemLibrary.DrawDebugSphere` _location 24.0 24 (select `bool` (`SceneComponent.bVisible` _hitcomponent) :`false` (struct :`R` 0.045745 :`G` 1.0 :`A` 1.0) :`true` (select `bool` _returnvalue_3 :`false` (struct :`R` 1.0 :`A` 1.0) :`true` (struct :`G` 0.163426 :`B` 1.0 :`A` 1.0) :!type "LinearColor Structure"))))))

(event `Remove Wall`
  (params (Maze :type "/Game/Procedural_Maze_Generator/Blueprints/MazeGenerator_BP Object Reference"))
  (bind _component (`self.Component`))
  (bind _cell (`self.Cell`))
  (bind _cell_parametrs (`/Game/Procedural_Maze_Generator/Blueprints/MazeGenerator_BP.Cell Parametrs` Maze))
  (bind _returnvalue (`KismetArrayLibrary.Array_Find` (`/Game/Procedural_Maze_Generator/Blueprints/MazeGenerator_BP.CellArray` Maze) (`self.Cell`)))
  (bind _output (`|GetArrayItem` _cell_parametrs _returnvalue))
  ;[1 1 1] Remove Wall (Edit Mode)
  (`/Engine/EditorBlueprintResources/StandardMacros.IsValid` _cell
    (:`Is Valid`
      (`/Engine/EditorBlueprintResources/StandardMacros.IsValid` _component
        (:`Is Valid`
          (`/Game/Procedural_Maze_Generator/Blueprints/Cell_BP.Set Visibility Wall` _cell _component false)
          (if (== _component (`/Game/Procedural_Maze_Generator/Blueprints/Cell_BP.Wall Left` _cell))
            (bind _structout (setmembers `/Game/Procedural_Maze_Generator/Blueprints/Cell_STR` :`StructRef` _output :`Wall Left` false))
            (`KismetArrayLibrary.Array_Set` _cell_parametrs _returnvalue _structout)
            (else
              (bind _structout_2 (setmembers `/Game/Procedural_Maze_Generator/Blueprints/Cell_STR` :`StructRef` _output :`Wall Back` false))
              (`KismetArrayLibrary.Array_Set` _cell_parametrs _returnvalue _structout_2))))))))

(event `Create Wall`
  (params (Maze :type "/Game/Procedural_Maze_Generator/Blueprints/MazeGenerator_BP Object Reference"))
  (bind _cell_parametrs (`/Game/Procedural_Maze_Generator/Blueprints/MazeGenerator_BP.Cell Parametrs` Maze))
  (bind _component (`self.Component`))
  (bind _cell (`self.Cell`))
  (bind _returnvalue (`KismetArrayLibrary.Array_Find` (`/Game/Procedural_Maze_Generator/Blueprints/MazeGenerator_BP.CellArray` Maze) (`self.Cell`)))
  (bind _output (`|GetArrayItem` _cell_parametrs _returnvalue))
  ;[1 1 1] Create Wall (Edit Mode)
  (`/Engine/EditorBlueprintResources/StandardMacros.IsValid` _cell
    (:`Is Valid`
      (`/Engine/EditorBlueprintResources/StandardMacros.IsValid` _component
        (:`Is Valid`
          (`/Game/Procedural_Maze_Generator/Blueprints/Cell_BP.Set Visibility Wall` _cell _component true)
          (if (== _component (`/Game/Procedural_Maze_Generator/Blueprints/Cell_BP.Wall Left` _cell))
            (bind _structout (setmembers `/Game/Procedural_Maze_Generator/Blueprints/Cell_STR` :`StructRef` _output :`Wall Left` true))
            (`KismetArrayLibrary.Array_Set` _cell_parametrs _returnvalue _structout)
            (else
              (bind _structout_2 (setmembers `/Game/Procedural_Maze_Generator/Blueprints/Cell_STR` :`StructRef` _output :`Wall Back` true))
              (`KismetArrayLibrary.Array_Set` _cell_parametrs _returnvalue _structout_2))))))))

(event `Place Exit`
  (params (Maze :type "/Game/Procedural_Maze_Generator/Blueprints/MazeGenerator_BP Object Reference"))
  (bind _preview_exit_cell (`self.Preview Exit Cell`))
  (bind _cell (`self.Cell`))
  ;[1 1 1] Place Exit (Edit Mode)
  (`/Engine/EditorBlueprintResources/StandardMacros.IsValid` _cell
    (:`Is Valid`
      (`/Engine/EditorBlueprintResources/StandardMacros.IsValid` _preview_exit_cell
        (:`Is Valid`
          (`/Game/Procedural_Maze_Generator/Blueprints/Cell_BP.Place Exit (Edit)` _preview_exit_cell false))
        (:`Is Not Valid`
          _))
      (`/Game/Procedural_Maze_Generator/Blueprints/Cell_BP.Place Exit (Edit)` _cell true)
      (set `self.Preview Exit Cell` _cell)
      (set `/Game/Procedural_Maze_Generator/Blueprints/MazeGenerator_BP.CellWithExit` (`KismetArrayLibrary.Array_Find` (`/Game/Procedural_Maze_Generator/Blueprints/MazeGenerator_BP.CellArray` Maze) (`self.Cell`)) Maze))))

(fn `UserConstructionScript`)