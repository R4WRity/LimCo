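; Cell_BP is one tile of the procedural maze, with a floor, left and back walls, a column and an exit trigger box.
; Delayed events use CellParametrs to remove unneeded parts and tint the start, exit and path floors through dynamic materials.
; When Maze_GM is in Edit mode, walls and columns are hidden rather than destroyed.
; SetVisibilityWall toggles walls along with the shared column, and Edit.PlaceExit recolours the floor as exit or plain.
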(event `Remove Component`
  (params (Duration :type "Float (double-precision)"))
  (bind _column (`self.Column`))
  (bind _wall_left (`self.Wall Left`))
  (bind _wall_back (`self.Wall Back`))
  (bind _floor (`self.Floor`))
  (bind ((`X_2_01B6F2724D21B49A8399809D59462664` _x) (`Y_4_2B2D8F664C7AB79EC4C77BA527DE226E` _y)) (break `/Game/Procedural_Maze_Generator/Blueprints/Cell_STR` (`self.Cell Parametrs`)))
  (bind ((`WallLeft_7_2690307D48F9E493D3D1AEAA61CECCFD` _wallleft) (`WallBack_11_B5C801164A70DBD6AA75ECB97FC9ADA0` _wallback) (`Floor_13_C3FDA05E4F4668413BF90FA32718C9B4` _floor_2)) (break `/Game/Procedural_Maze_Generator/Blueprints/Cell_STR` (`self.Cell Parametrs`)))
  (`KismetSystemLibrary.Delay` Duration)
  (if (not _wallleft)
    (`/Engine/EditorBlueprintResources/StandardMacros.IsValid` _wall_left
      (:`Is Valid`
        (if (`/Game/Procedural_Maze_Generator/Blueprints/Maze_GM.Edit` (cast `/Game/Procedural_Maze_Generator/Blueprints/Maze_GM` (`GameplayStatics.GetGameMode`) :!pure true))
          (`SceneComponent.SetVisibility` _wall_left false false)
          (else
            (`ActorComponent.K2_DestroyComponent` _wall_left))))
      (:`Is Not Valid`
        _)))
  (if (not _wallback)
    (`/Engine/EditorBlueprintResources/StandardMacros.IsValid` _wall_back
      (:`Is Valid`
        (if (`/Game/Procedural_Maze_Generator/Blueprints/Maze_GM.Edit` (cast `/Game/Procedural_Maze_Generator/Blueprints/Maze_GM` (`GameplayStatics.GetGameMode`) :!pure true))
          (`SceneComponent.SetVisibility` _wall_back false false)
          (else
            (`ActorComponent.K2_DestroyComponent` _wall_back))))
      (:`Is Not Valid`
        _)))
  (if (not _floor_2)
    (`/Engine/EditorBlueprintResources/StandardMacros.IsValid` _floor
      (:`Is Valid`
        (`ActorComponent.K2_DestroyComponent` _floor))
      (:`Is Not Valid`
        _)))
  (if (and (not _wallleft) (not _wallback))
    (if (`/Game/Procedural_Maze_Generator/Blueprints/Maze_GM.Edit` (cast `/Game/Procedural_Maze_Generator/Blueprints/Maze_GM` (`GameplayStatics.GetGameMode`) :!pure true))
      (`SceneComponent.SetVisibility` _column false false)
      (else
        (`/Engine/EditorBlueprintResources/StandardMacros.IsValid` _column
          (:`Is Valid`
            (`ActorComponent.K2_DestroyComponent` _column))
          (:`Is Not Valid`
            _)))))
  ;[1 1 1] Start
  (if (and (== _x 0) (== _y 0))
    (bind _returnvalue (`PrimitiveComponent.CreateDynamicMaterialInstance` (`self.Floor`) 0 (`PrimitiveComponent.GetMaterial` (`self.Floor`) 0) "None"))
    (`MaterialInstanceDynamic.SetVectorParameterValue` _returnvalue "Color" (struct :`G` 0.403831 :`B` 1.0 :`A` 1.0))))

(event `Place Exit`
  (params (Duration :type "Float (double-precision)"))
  (bind _triggerbox (`self.TriggerBox`))
  (if (`.Exit_23_46A598ED4A47DE0A2487D5A8EDA4436C` (break `/Game/Procedural_Maze_Generator/Blueprints/Cell_STR` (`self.Cell Parametrs`)))
    (`KismetSystemLibrary.Delay` Duration)
    ;[1 1 1] Exit
    (bind _returnvalue (`PrimitiveComponent.CreateDynamicMaterialInstance` (`self.Floor`) 0 (`PrimitiveComponent.GetMaterial` (`self.Floor`) 0) "None"))
    (`MaterialInstanceDynamic.SetVectorParameterValue` _returnvalue "Color" (struct :`R` 1.0 :`B` 0.109699 :`A` 1.0))
    (else
      (`/Engine/EditorBlueprintResources/StandardMacros.IsValid` _triggerbox
        (:`Is Valid`
          (`ActorComponent.K2_DestroyComponent` _triggerbox))))))

(event `Set Visibility Wall`
  (params (Wall :type "SceneComponent Object Reference") (Visibility :type Boolean))
  (bind _returnvalue (not Visibility))
  (bind _returnvalue_2 (== Wall (`self.Column`)))
  (bind _returnvalue_3 (`SceneComponent.IsVisible` (`self.Wall Back`)))
  (bind _returnvalue_4 (`SceneComponent.IsVisible` (`self.Wall Left`)))
  (bind _returnvalue_5 (not _returnvalue_4))
  (bind _returnvalue_6 (not _returnvalue_3))
  (bind _returnvalue_7 (and _returnvalue_6 _returnvalue_4))
  (bind _returnvalue_8 (and _returnvalue_6 _returnvalue_5 (not (`SceneComponent.IsVisible` (`self.Column`)))))
  (bind _returnvalue_9 (or _returnvalue_7 (and _returnvalue_3 _returnvalue_5)))
  ;[1 1 1] Set Visibility Wall
  (if _returnvalue_2
    (if _returnvalue
      (if (and _returnvalue_2 _returnvalue_9)
        (`SceneComponent.SetVisibility` (select `bool` _returnvalue_7 :`false` (`self.Wall Back`) :`true` (`self.Wall Left`) :!type "SceneComponent Object Reference") false false)
        (`SceneComponent.SetVisibility` (`self.Column`) false false)
        (else
          (`SceneComponent.SetVisibility` (`self.Wall Back`) false false)))
      (elif _returnvalue_8
        (`SceneComponent.SetVisibility` (`self.Column`) true false)
        (`SceneComponent.SetVisibility` (`self.Wall Back`) true false)))
    (elif _returnvalue
      (if _returnvalue_9
        (`SceneComponent.SetVisibility` Wall false false)
        (`SceneComponent.SetVisibility` (`self.Column`) false false)
        (else
          (`SceneComponent.SetVisibility` Wall false false)))
      (elif _returnvalue_8
        (`SceneComponent.SetVisibility` Wall true false)
        (`SceneComponent.SetVisibility` (`self.Column`) true false)
        (else
          (`SceneComponent.SetVisibility` Wall true false))))))

(event `Mark Path`
  (params (Duration :type "Float (double-precision)"))
  (bind ((`X_2_01B6F2724D21B49A8399809D59462664` _x) (`Y_4_2B2D8F664C7AB79EC4C77BA527DE226E` _y)) (break `/Game/Procedural_Maze_Generator/Blueprints/Cell_STR` (`self.Cell Parametrs`)))
  ;[1 1 1] Mark Path
  (if (not (`.Exit_23_46A598ED4A47DE0A2487D5A8EDA4436C` (break `/Game/Procedural_Maze_Generator/Blueprints/Cell_STR` (`self.Cell Parametrs`))))
    (`KismetSystemLibrary.Delay` Duration)
    (if (not (and (== _x 0) (== _y 0)))
      (bind _returnvalue (`PrimitiveComponent.CreateDynamicMaterialInstance` (`self.Floor`) 0 (`PrimitiveComponent.GetMaterial` (`self.Floor`) 0) "None"))
      (`MaterialInstanceDynamic.SetVectorParameterValue` _returnvalue "Color" (struct :`R` 0.040498 :`G` 1.0 :`A` 1.0)))))

(event `self.TriggerBox.OnComponentBeginOverlap`
  (params (OverlappedComponent :type "PrimitiveComponent Object Reference") (OtherActor :type "Actor Object Reference") (OtherComp :type "PrimitiveComponent Object Reference") (OtherBodyIndex :type Integer) (bFromSweep :type Boolean) (SweepResult :type "HitResult Structure (by ref)"))
  ;[1 1 1] Exit
)

(event `Place Exit (Edit)`
  (params (`Exit?` :type Boolean))
  (bind _triggerbox (`self.TriggerBox`))
  (if `Exit?`
    (bind _returnvalue (`PrimitiveComponent.CreateDynamicMaterialInstance` (`self.Floor`) 0 (`PrimitiveComponent.GetMaterial` (`self.Floor`) 0) "None"))
    (`MaterialInstanceDynamic.SetVectorParameterValue` _returnvalue "Color" (struct :`R` 1.0 :`B` 0.109699 :`A` 1.0))
    (else
      (bind _returnvalue_2 (`PrimitiveComponent.CreateDynamicMaterialInstance` (`self.Floor`) 0 (`PrimitiveComponent.GetMaterial` (`self.Floor`) 0) "None"))
      (`MaterialInstanceDynamic.SetVectorParameterValue` _returnvalue_2 "Color" (struct :`R` 0.180392 :`G` 0.180392 :`B` 0.180392))
      (`/Engine/EditorBlueprintResources/StandardMacros.IsValid` _triggerbox
        (:`Is Valid`
          (`ActorComponent.K2_DestroyComponent` _triggerbox))))))

(fn `UserConstructionScript`)